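; RayBP fires a reflected electric ray from its Scene component toward a target actor's location.
; On BeginPlay it binds FireRay to a fire event, and FireRay calls Shoot on Reflected with a fixed trace length and color.
; The returned distance divided by Speed sets a delay, after which it calls FireDone to signal completion after the travel time.
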(event `self.ReceiveBeginPlay`
  (add `self.Fire` (delegate `FireRay`)))

(event `FireRay`
  (bind (_ishit _distance) (`/Game/ReflectedElectricity/Blueprints/Reflected.Shoot` (`self.Reflected`) 5000.0 (`self.Scene`) "NewEnumerator0" (`self.K2_GetActorLocation` (`self.TargetActor`))))
  (`KismetSystemLibrary.Delay` (/ _distance (`self.speed`)))
  (`self.FireDone`))

(fn `UserConstructionScript`)