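; Reflected fires colored electric beam effects and computes where they would bounce off surfaces.
; Shoot line-traces forward on Visibility, stores a mirrored second segment from the impact normal, and returns hit and distance.
; It spawns a color-selected beam emitter from the source component to the supplied target position, regardless of the hit, and records it in an array.
; Clear destroys the stored emitters and empties that array.
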(fn `Clear`
  (bind _particlearray (`self.ParticleArray`))
  ;[1 1 1] Here , we are getting our Beam Array which we store in our Reflect function , first we destroy it and we clear the array afterwards.
  (`self.K2_DestroyComponent` _particlearray)
  (`KismetArrayLibrary.Array_Clear` _particlearray))

(fn `Shoot`
  (params (TraceLength :type "Float (double-precision)") (ShootFrom :type "SceneComponent Object Reference") (Color :type "/Game/ReflectedElectricity/Blueprints/E_Colors Enum" :default "NewEnumerator0") (TargetPosition :type "Vector Structure"))
  (returns (IsHit :type Boolean) (Distance :type "Float (double-precision)"))
  (locals (SecondHitStart :type "Vector Structure") (SecondHitEnd :type "Vector Structure") (LoopStart :type "Vector Structure") (HResult :type "HitResult Structure"))
  (bind _returnvalue (`SceneComponent.K2_GetComponentLocation` ShootFrom))
  (bind (_outhit _returnvalue_2) (`KismetSystemLibrary.LineTraceSingle` _returnvalue (+ (* (`SceneComponent.GetForwardVector` ShootFrom) TraceLength) _returnvalue) "TraceTypeQuery1" true))
  (if _returnvalue_2
    _
    (else
      _))
  (bind (_bblockinghit _binitialoverlap _time _distance _location _impactpoint _normal _impactnormal _physmat _hitactor _hitcomponent _hitbonename _hititem _faceindex _tracestart _traceend) (`GameplayStatics.BreakHitResult` _outhit))
  (set `local.SecondHitStart` (+ _impactpoint _normal))
  (set `local.SecondHitEnd` (+ _impactpoint (`KismetMathLibrary.MirrorVectorByNormal` (- _traceend _tracestart) _impactnormal)))
  (bind _returnvalue_3 (`GameplayStatics.SpawnEmitterAtLocation` (select `/Game/ReflectedElectricity/Blueprints/E_Colors` Color :`NewEnumerator0` "/Game/ReflectedElectricity/Particles/P_ElectricWhite.P_ElectricWhite" :`NewEnumerator1` "/Game/ReflectedElectricity/Particles/P_ElectricBlue.P_ElectricBlue" :`NewEnumerator2` "/Game/ReflectedElectricity/Particles/P_ElectricRed.P_ElectricRed" :`NewEnumerator3` "/Game/ReflectedElectricity/Particles/P_ElectricGreen.P_ElectricGreen" :`NewEnumerator4` "/Game/ReflectedElectricity/Particles/P_ElectricPurple.P_ElectricPurple" :!type "ParticleSystem Object Reference")))
  (`ParticleSystemComponent.SetBeamSourcePoint` _returnvalue_3 0 (`SceneComponent.K2_GetComponentLocation` ShootFrom) 0)
  (`ParticleSystemComponent.SetBeamEndPoint` _returnvalue_3 0 TargetPosition)
  (`KismetArrayLibrary.Array_Add` (`self.ParticleArray`) _returnvalue_3)
  (return _bblockinghit _distance))